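; BP_Vaisseau is a ship that turns to face the mouse cursor and fires on player input.
; Every tick it traces under the cursor on the Visibility channel and looks at the hit point, using its own Z height so it only yaws.
; The Tir input press calls a Tir function whose body is not in this graph.
; An older look-at without the height flattening remains unconnected.
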(event `InputAction|Tir`
  (params (Key :type "Key Structure"))
  (:`Pressed`
    (`self.Tir`)))

(event `self.ReceiveBeginPlay`)

(event `self.ReceivePossessed`
  (params (NewController :type "Controller Object Reference")))

(event `self.ReceiveTick`
  (params (DeltaSeconds :type "Float (single-precision)"))
  (`self.K2_SetActorRotation` (`KismetMathLibrary.FindLookAtRotation` (`self.K2_GetActorLocation`) (`KismetMathLibrary.MakeVector` (.x (`.ImpactPoint` (`GameplayStatics.BreakHitResult` (`PlayerController.GetHitResultUnderCursorByChannel` (`GameplayStatics.GetPlayerController` 0) "TraceTypeQuery1" true)))) (.y (`.ImpactPoint` (`GameplayStatics.BreakHitResult` (`PlayerController.GetHitResultUnderCursorByChannel` (`GameplayStatics.GetPlayerController` 0) "TraceTypeQuery1" true)))) (.z (`self.K2_GetActorLocation` self))))))

(fn `UserConstructionScript`)